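; First-person survival player character handling Enhanced Input movement, sprinting, inventory, crafting, building and harvesting.
; Tick uses Delay-throttled branches to drain and regenerate stamina and deplete food and water, with hunger or thirst blocking regeneration.
; Input drives the InventoryManager's hotbar, item use and drops, plus BPBuildComponent's ghost selection, rotation and placement.
; Mine_Button line-traces to toggle storage chests and destroy tagged trees, rocks or pigs, spawning random resource drops.
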(event `EnhancedInput|/Game/FP_Player/Input/Mine_Button`
  (params (ActionValue :type Boolean) (ElapsedSeconds :type "Float (double-precision)") (TriggeredSeconds :type "Float (double-precision)") (InputAction :type "InputAction Object Reference" :default "/Game/FP_Player/Input/Mine_Button.Mine_Button"))
  (bind _returnvalue (`SceneComponent.K2_GetComponentLocation` (`self.Camera`)))
  (:`Started`
    (bind (_outhit _returnvalue_2) (`KismetSystemLibrary.LineTraceSingle` :`Start` _returnvalue :`End` (+ _returnvalue (* (`KismetMathLibrary.GetForwardVector` (`KismetMathLibrary.MakeRotator` 0.0 (.pitch (`SceneComponent.K2_GetComponentRotation` (`self.Camera`))) (.yaw (`SceneComponent.K2_GetComponentRotation` (`self.Camera`))))) 300.0)) :`TraceChannel` "TraceTypeQuery1" :`DrawDebugType` "Persistent"))
    (if _returnvalue_2
      (`KismetSystemLibrary.Delay` 0.5)
      (bind (_bblockinghit _binitialoverlap _time _distance _location _impactpoint _normal _impactnormal _physmat _hitactor) (`GameplayStatics.BreakHitResult` _outhit))
      (bind (_tag _actor_out) (`self.tag checker` _hitactor))
      (switch `name` _tag
        (:`Tree`
          (bind _returnvalue_3 (`KismetMathLibrary.MakeTransform` _impactpoint))
          (`self.destroy tree` _returnvalue_3 _actor_out))
        (:`Rock`
          (`self.Destroy Rock` _returnvalue_3 _actor_out))
        (:`Pig`
          (`self.Destroy Pig` _returnvalue_3 _actor_out))))))

(event `self.ReceiveBeginPlay`
  (set `/Game/Build/Export/BP_Build_Component.cam` (`self.Camera`) (`self.BP_Build_Component`))
  ;[1 1 1] Stamina UI
  (`WidgetBlueprintLibrary.SetInputMode_GameOnly` (`GameplayStatics.GetPlayerController` 0))
  (bind _returnvalue (`|CreateWidget` "/Game/Widigts/StaminaWidget.StaminaWidget_C"))
  (`UserWidget.AddToViewport` _returnvalue 0)
  ;[1 1 1] Add button Mapping
  (bind _asplayer_controller (cast `PlayerController` (`self.GetController`)))
  (bind _returnvalue_2 (pcsubsystem `EnhancedInputLocalPlayerSubsystem` _asplayer_controller))
  (`/Engine/EditorBlueprintResources/StandardMacros.IsValid` _returnvalue_2
    (:`Is Valid`
      (`EnhancedInputSubsystemInterface.AddMappingContext` _returnvalue_2 "/Game/FP_Player/Input/Player_InputMapping.Player_InputMapping" 0 (struct))
      ;[1 1 1] Inventory System code
      ;;[1 1 1] Get & Set the inventory manager
      (bind _inventorymanagercomponent (`/Game/InventorySystem/Blueprints/BPFL_InventoryFunctionLib.GetInventoryManager` self))
      (set `self.InventoryManager` _inventorymanagercomponent))))

(event `EnhancedInput|/Game/FP_Player/Input/Look_Axis`
  (params (ActionValue :type "Vector2D Structure") (ElapsedSeconds :type "Float (double-precision)") (TriggeredSeconds :type "Float (double-precision)") (InputAction :type "InputAction Object Reference" :default "/Game/FP_Player/Input/Look_Axis.Look_Axis"))
  ;[1 1 1] Look
  (:`Triggered`
    (`self.AddControllerYawInput` ActionValue_X)
    (bind _result (`/Engine/EditorBlueprintResources/StandardMacros.NegateFloat` ActionValue_Y)
      (:`  `
        (`self.AddControllerPitchInput` _result)))))

(event `EnhancedInput|/Game/FP_Player/Input/InventoryToggle`
  (params (ActionValue :type Boolean) (ElapsedSeconds :type "Float (double-precision)") (TriggeredSeconds :type "Float (double-precision)") (InputAction :type "InputAction Object Reference" :default "/Game/FP_Player/Input/InventoryToggle.InventoryToggle"))
  (:`Started`
    ;[1 1 1] Inventory System code
    ;;[1 1 1] Toggle if the inventory is open or not!
    (`/Game/InventorySystem/Blueprints/BP_InventoryManagerComponent.ToggleInventoryOpen` (`self.InventoryManager`))
    ;;[1 1 1] Gain and Loose control over the character. In  here to save a cast!
    (set `self.IsBeingControlled?` (not (`self.IsBeingControlled?`)))))

(event `self.ReceiveTick`
  (params (DeltaSeconds :type "Float (single-precision)"))
  (`|ExecutionSequence`
    (:`then_0`
      ;[1 1 1] Stamina Drain
      (if (and (`self.Is Sprinting`) (`self.move forward`))
        (if (> (`self.Stamina`) 0)
          (`KismetSystemLibrary.Delay` 0.1)
          (set `self.Stamina` (`KismetMathLibrary.Clamp` (- (`self.Stamina`) 1) 0 (`self.Max Stamina`)))
          (else
            (`self.Stop Sprinting`)))))
    (:`then_1`
      ;[1 1 1] Stamina Replanish
      (if (`self.CanRegen`)
        (if (`self.move forward`)
          _
          (elif (< (`self.Stamina`) (`self.Max Stamina`))
            (`KismetSystemLibrary.Delay` 0.5)
            (set `self.Stamina` (`KismetMathLibrary.Clamp` (+ (`self.Stamina`) 5) 0 (`self.Max Stamina`)))))))
    (:`then_2`
      (if (or (`self.Thirst`) (`self.Hunger`))
        (set `self.CanRegen` false)
        (else
          (set `self.CanRegen` true)
          (`KismetSystemLibrary.Delay` (`KismetMathLibrary.RandomFloatInRange` 3.0 12.0))
          (bind _output_get (set `self.water` (`KismetMathLibrary.Clamp` (- (`self.water`) (`KismetMathLibrary.RandomIntegerInRange` 1 5)) 0 (`self.MaxWater`))))
          (`KismetSystemLibrary.PrintString` (`KismetStringLibrary.Conv_IntToString` _output_get)))))
    (:`then_3`
      (if (== (`self.water`) 0)
        (set `self.Thirst` true)
        (else
          (set `self.Thirst` false))))
    (:`then_4`
      (`|ExecutionSequence`
        (:`then_2`
          (if (or (`self.Thirst`) (`self.Hunger`))
            (set `self.CanRegen` false)
            (else
              (set `self.CanRegen` true)
              (`KismetSystemLibrary.Delay` (`KismetMathLibrary.RandomFloatInRange` 3.0 12.0))
              (bind _output_get_2 (set `self.Fod` (`KismetMathLibrary.Clamp` (- (`self.Fod`) (`KismetMathLibrary.RandomIntegerInRange` 1 5)) 0 (`self.MaxFod`))))
              (`KismetSystemLibrary.PrintString` (`KismetStringLibrary.Conv_IntToString` _output_get_2)))))
        (:`then_3`
          (if (== (`self.Fod`) 0)
            (set `self.Hunger` true)
            (else
              (set `self.Hunger` false))))))))

(event `EnhancedInput|/Game/FP_Player/Input/Mouse_use`
  (params (ActionValue :type Boolean) (ElapsedSeconds :type "Float (double-precision)") (TriggeredSeconds :type "Float (double-precision)") (InputAction :type "InputAction Object Reference" :default "/Game/FP_Player/Input/Mouse_use.Mouse_use"))
  ;[1 1 1] Inventory System code
  ;;[1 1 1] Code for using an item in the selected hotbar slot (use RMB to use an item)
  (:`Triggered`
    (if (`self.IsBeingControlled?`)
      (`/Game/InventorySystem/Blueprints/BP_InventoryManagerComponent.DoUseItem` (`self.InventoryManager`)))))

(event `EnhancedInput|/Game/FP_Player/Input/CraftToggle`
  (params (ActionValue :type Boolean) (ElapsedSeconds :type "Float (double-precision)") (TriggeredSeconds :type "Float (double-precision)") (InputAction :type "InputAction Object Reference" :default "/Game/FP_Player/Input/CraftToggle.CraftToggle"))
  (:`Started`
    ;[1 1 1] Inventory System code
    ;;[1 1 1] Toggle if the inventory is open or not!
    (`/Game/InventorySystem/Blueprints/BP_InventoryManagerComponent.ToggleCraftingDisplayOpen` (`self.InventoryManager`))
    ;;[1 1 1] Gain and Loose control over the character. In  here to save a cast!
    (set `self.IsBeingControlled?` (not (`self.IsBeingControlled?`)))))

(event `EnhancedInput|/Game/FP_Player/Input/Move_Axis`
  (params (ActionValue :type "Vector2D Structure") (ElapsedSeconds :type "Float (double-precision)") (TriggeredSeconds :type "Float (double-precision)") (InputAction :type "InputAction Object Reference" :default "/Game/FP_Player/Input/Move_Axis.Move_Axis"))
  ;[1 1 1] Movement
  (:`Triggered`
    (if (not (`self.Openchest`))
      (`self.AddMovementInput` (`self.GetActorRightVector`) ActionValue_X)
      (`self.AddMovementInput` (`self.GetActorForwardVector`) ActionValue_Y)
      ;[1 1 1] MoveCheck
      (set `self.move forward` true)
      (if (and (`self.move forward`) (`self.playwalk`)) :!label _label
        (set `self.playwalk` false)
        (`GameplayStatics.PlaySoundAtLocation` "/Game/Sound/footsteps-1.footsteps-1" (`SceneComponent.K2_GetComponentLocation` (`self.FP_Player_Mesh`)) (struct) 1.0 1.0 0.0 null null null null)
        (`KismetSystemLibrary.Delay` 0.5)
        (set `self.playwalk` true)
        (if (and (`self.move forward`) (`self.playwalk`))
          (set `self.playwalk` false)
          (`GameplayStatics.PlaySoundAtLocation` "/Game/Sound/footsteps-1.footsteps-1" (`SceneComponent.K2_GetComponentLocation` (`self.FP_Player_Mesh`)) (struct) 1.0 1.0 0.0 null null null null)
          (`KismetSystemLibrary.Delay` 0.5)
          (set `self.playwalk` true)
          (goto _label)))))
  (:`Started`
    (set `self.playwalk` true))
  (:`Completed`
    (set `self.move forward` false)))

(event `EnhancedInput|/Game/FP_Player/Input/Jump_Button`
  (params (ActionValue :type Boolean) (ElapsedSeconds :type "Float (double-precision)") (TriggeredSeconds :type "Float (double-precision)") (InputAction :type "InputAction Object Reference" :default "/Game/FP_Player/Input/Jump_Button.Jump_Button"))
  ;[1 1 1] Jumping
  (:`Triggered`
    (`self.Jump`))
  (:`Completed`
    (`self.StopJumping`)))

(event `EnhancedInput|/Game/FP_Player/Input/Spritn_Button`
  (params (ActionValue :type Boolean) (ElapsedSeconds :type "Float (double-precision)") (TriggeredSeconds :type "Float (double-precision)") (InputAction :type "InputAction Object Reference" :default "/Game/FP_Player/Input/Spritn_Button.Spritn_Button"))
  ;[1 1 1] sprinting
  (:`Triggered`
    (`self.Start Sprinting` :!label _label_2))
  (:`Ongoing`
    (goto _label_2))
  (:`Canceled`
    (`self.Stop Sprinting` :!label _label_3))
  (:`Completed`
    (goto _label_3)))

(event `EnhancedInput|/Game/FP_Player/Input/InvScroll`
  (params (ActionValue :type "Float (double-precision)") (ElapsedSeconds :type "Float (double-precision)") (TriggeredSeconds :type "Float (double-precision)") (InputAction :type "InputAction Object Reference" :default "/Game/FP_Player/Input/InvScroll.InvScroll"))
  (bind _bp_build_component (`self.BP_Build_Component`))
  (bind (_buildtransform_location _buildtransform_rotation _buildtransform_scale) (`KismetMathLibrary.BreakTransform` (`/Game/Build/Export/BP_Build_Component.buildTransform` _bp_build_component)))
  (:`Triggered`
    (`|ExecutionSequence`
      (:`then_0`
        (goto _label_4 :!via `Open`))
      (:`then_1`
        (if true
          (`/Engine/EditorBlueprintResources/StandardMacros.Gate` true :!label _label_4
            (:`Exit`
              (set `/Game/Build/Export/BP_Build_Component.buildTransform` (`KismetMathLibrary.MakeTransform` _buildtransform_location (`KismetMathLibrary.ComposeRotators` _buildtransform_rotation (struct :`Yaw` 2.5)) _buildtransform_scale) _bp_build_component)))))))
  (:`Canceled`
    (goto _label_4 :!via `Close`)))

(event `Key|Q`
  (params (Key :type "Key Structure"))
  (:`Pressed`
    (`/Engine/EditorBlueprintResources/StandardMacros.FlipFlop`
      (:`A`
        (`KismetSystemLibrary.PrintString` "BUILD ON" true true (struct :`R` 1.0 :`B` 0.030547 :`A` 1.0))
        (`/Game/Build/Export/BP_Build_Component.LaunchBuildMode` (`self.BP_Build_Component`)))
      (:`B`
        (`KismetSystemLibrary.PrintString` "BUILLD OFF" true true (struct :`R` 0.009027 :`G` 1.0 :`A` 1.0))))))

(event `Key|V`
  (params (Key :type "Key Structure"))
  (bind _bp_build_component (`self.BP_Build_Component`))
  (:`Pressed`
    (if (and (`/Game/Build/Export/BP_Build_Component.isBuildModeOn` _bp_build_component) (`/Game/Build/Export/BP_Build_Component.canBuild` _bp_build_component))
      (`/Game/Build/Export/BP_Build_Component.Spawn Build` (`self.BP_Build_Component`)))))

(event `EnhancedInput|/Game/FP_Player/Input/Interact_Button`
  (params (ActionValue :type Boolean) (ElapsedSeconds :type "Float (double-precision)") (TriggeredSeconds :type "Float (double-precision)") (InputAction :type "InputAction Object Reference" :default "/Game/FP_Player/Input/Interact_Button.Interact_Button"))
  (:`Started`
    (set `self.Interact?` true)
    (`KismetSystemLibrary.PrintString` "on"))
  (:`Completed`
    (set `self.Interact?` false)
    (`KismetSystemLibrary.PrintString` "off")))

(event `EnhancedInput|/Game/FP_Player/Input/Up`
  (params (ActionValue :type Boolean) (ElapsedSeconds :type "Float (double-precision)") (TriggeredSeconds :type "Float (double-precision)") (InputAction :type "InputAction Object Reference" :default "/Game/FP_Player/Input/Up.Up"))
  (bind _bp_build_component (`self.BP_Build_Component`))
  (bind _bp_build_component_2 (`self.BP_Build_Component`))
  (bind _bp_build_component_3 (`self.BP_Build_Component`))
  (:`Triggered`
    (if (and (`/Game/Build/Export/BP_Build_Component.isBuildModeOn` _bp_build_component) (`KismetSystemLibrary.IsValid` (`/Game/Build/Export/BP_Build_Component.buildGhost` _bp_build_component)))
      (set `/Game/Build/Export/BP_Build_Component.buildID` (`KismetMathLibrary.Clamp` (+ (`/Game/Build/Export/BP_Build_Component.buildID` _bp_build_component_2) 1) 0 (- (`KismetArrayLibrary.Array_Length` (`/Game/Build/Export/BP_Build_Component.buildables` _bp_build_component_2)) 1)) _bp_build_component_3)
      (`/Game/Build/Export/BP_Build_Component.ChangeMesh` _bp_build_component_3 :!label _label_5))))

(event `EnhancedInput|/Game/FP_Player/Input/Down`
  (params (ActionValue :type Boolean) (ElapsedSeconds :type "Float (double-precision)") (TriggeredSeconds :type "Float (double-precision)") (InputAction :type "InputAction Object Reference" :default "/Game/FP_Player/Input/Down.Down"))
  (bind _bp_build_component (`self.BP_Build_Component`))
  (bind _bp_build_component_2 (`self.BP_Build_Component`))
  (:`Triggered`
    (if (and (`/Game/Build/Export/BP_Build_Component.isBuildModeOn` _bp_build_component) (`KismetSystemLibrary.IsValid` (`/Game/Build/Export/BP_Build_Component.buildGhost` _bp_build_component)))
      (set `/Game/Build/Export/BP_Build_Component.buildID` (`KismetMathLibrary.Clamp` (- (`/Game/Build/Export/BP_Build_Component.buildID` _bp_build_component_2) 1) 0 (- (`KismetArrayLibrary.Array_Length` (`/Game/Build/Export/BP_Build_Component.buildables` _bp_build_component_2)) 1)) (`self.BP_Build_Component`))
      (goto _label_5))))

(event `EnhancedInput|/Game/FP_Player/Input/Mine_Button`
  (params (ActionValue :type Boolean) (ElapsedSeconds :type "Float (double-precision)") (TriggeredSeconds :type "Float (double-precision)") (InputAction :type "InputAction Object Reference" :default "/Game/FP_Player/Input/Mine_Button.Mine_Button"))
  (bind _camera (`self.Camera`))
  (bind _returnvalue (`SceneComponent.K2_GetComponentLocation` _camera))
  (:`Started`
    ;[1 1 1] Is there a chest that the user has currently opened?
    (`/Engine/EditorBlueprintResources/StandardMacros.IsValid` (`self.CurrentlyOpenChest`)
      (:`Is Valid`
        ;[1 1 1] Close the chest by toggling it, and then setting the reference to none/null (so it won't think it is still open)
        (`/Game/InventorySystem/Blueprints/BP_StorageChest.ToggleChest` (`self.CurrentlyOpenChest`))
        (set `self.CurrentlyOpenChest` null)
        (set `self.Openchest` false))
      (:`Is Not Valid`
        (bind _outhit (`KismetSystemLibrary.LineTraceSingle` _returnvalue (+ (* (`SceneComponent.GetForwardVector` _camera) (`self.ChestOpenReach`)) _returnvalue) "TraceTypeQuery1"))
        (bind _asbp_storage_chest (cast `/Game/InventorySystem/Blueprints/BP_StorageChest` (`.HitActor` (`GameplayStatics.BreakHitResult` _outhit))))
        (`/Game/InventorySystem/Blueprints/BP_StorageChest.ToggleChest` _asbp_storage_chest)
        ;[1 1 1] Set the reference so we can later close this one
        (set `self.CurrentlyOpenChest` _asbp_storage_chest)
        (set `self.Openchest` true)))))

(event `Key|One`
  (params (Key :type "Key Structure"))
  ;[1 1 1] The hotbar controls to operate everything to do with the hotbar!!!
  ;;[1 1 1] Handle 1-9 to select hotbar slots!
  (:`Pressed`
    (`/Game/InventorySystem/UMG/WBP_HotbarWidget.SetSelectedSlot` (`/Game/InventorySystem/Blueprints/BP_InventoryManagerComponent.HotbarWidget` (`self.InventoryManager`)) 0)))

(event `Key|Six`
  (params (Key :type "Key Structure"))
  ;[1 1 1] The hotbar controls to operate everything to do with the hotbar!!!
  ;;[1 1 1] Handle 1-9 to select hotbar slots!
  (:`Pressed`
    (`/Game/InventorySystem/UMG/WBP_HotbarWidget.SetSelectedSlot` (`/Game/InventorySystem/Blueprints/BP_InventoryManagerComponent.HotbarWidget` (`self.InventoryManager`)) 5)))

(event `Key|Two`
  (params (Key :type "Key Structure"))
  ;[1 1 1] The hotbar controls to operate everything to do with the hotbar!!!
  ;;[1 1 1] Handle 1-9 to select hotbar slots!
  (:`Pressed`
    (`/Game/InventorySystem/UMG/WBP_HotbarWidget.SetSelectedSlot` (`/Game/InventorySystem/Blueprints/BP_InventoryManagerComponent.HotbarWidget` (`self.InventoryManager`)) 1)))

(event `Key|Seven`
  (params (Key :type "Key Structure"))
  ;[1 1 1] The hotbar controls to operate everything to do with the hotbar!!!
  ;;[1 1 1] Handle 1-9 to select hotbar slots!
  (:`Pressed`
    (`/Game/InventorySystem/UMG/WBP_HotbarWidget.SetSelectedSlot` (`/Game/InventorySystem/Blueprints/BP_InventoryManagerComponent.HotbarWidget` (`self.InventoryManager`)) 6)))

(event `Key|Three`
  (params (Key :type "Key Structure"))
  ;[1 1 1] The hotbar controls to operate everything to do with the hotbar!!!
  ;;[1 1 1] Handle 1-9 to select hotbar slots!
  (:`Pressed`
    (`/Game/InventorySystem/UMG/WBP_HotbarWidget.SetSelectedSlot` (`/Game/InventorySystem/Blueprints/BP_InventoryManagerComponent.HotbarWidget` (`self.InventoryManager`)) 2)))

(event `Key|Eight`
  (params (Key :type "Key Structure"))
  ;[1 1 1] The hotbar controls to operate everything to do with the hotbar!!!
  ;;[1 1 1] Handle 1-9 to select hotbar slots!
  (:`Pressed`
    (`/Game/InventorySystem/UMG/WBP_HotbarWidget.SetSelectedSlot` (`/Game/InventorySystem/Blueprints/BP_InventoryManagerComponent.HotbarWidget` (`self.InventoryManager`)) 7)))

(event `Key|Four`
  (params (Key :type "Key Structure"))
  ;[1 1 1] The hotbar controls to operate everything to do with the hotbar!!!
  ;;[1 1 1] Handle 1-9 to select hotbar slots!
  (:`Pressed`
    (`/Game/InventorySystem/UMG/WBP_HotbarWidget.SetSelectedSlot` (`/Game/InventorySystem/Blueprints/BP_InventoryManagerComponent.HotbarWidget` (`self.InventoryManager`)) 3)))

(event `Key|Nine`
  (params (Key :type "Key Structure"))
  ;[1 1 1] The hotbar controls to operate everything to do with the hotbar!!!
  ;;[1 1 1] Handle 1-9 to select hotbar slots!
  (:`Pressed`
    (`/Game/InventorySystem/UMG/WBP_HotbarWidget.SetSelectedSlot` (`/Game/InventorySystem/Blueprints/BP_InventoryManagerComponent.HotbarWidget` (`self.InventoryManager`)) 8)))

(event `Key|Five`
  (params (Key :type "Key Structure"))
  ;[1 1 1] The hotbar controls to operate everything to do with the hotbar!!!
  ;;[1 1 1] Handle 1-9 to select hotbar slots!
  (:`Pressed`
    (`/Game/InventorySystem/UMG/WBP_HotbarWidget.SetSelectedSlot` (`/Game/InventorySystem/Blueprints/BP_InventoryManagerComponent.HotbarWidget` (`self.InventoryManager`)) 4)))

(event `EnhancedInput|/Game/FP_Player/Input/InvScroll`
  (params (ActionValue :type "Float (double-precision)") (ElapsedSeconds :type "Float (double-precision)") (TriggeredSeconds :type "Float (double-precision)") (InputAction :type "InputAction Object Reference" :default "/Game/FP_Player/Input/InvScroll.InvScroll"))
  (bind _returnvalue (`KismetMathLibrary.FTrunc` (`self.GetInputAxisKeyValue`)))
  (bind _hotbarwidget (`/Game/InventorySystem/Blueprints/BP_InventoryManagerComponent.HotbarWidget` (`self.InventoryManager`)))
  ;[1 1 1] The hotbar controls to operate everything to do with the hotbar!!!
  ;;[1 1 1] Do the scrollwheel for hotbar slots!
  (:`Triggered`
    ;;;[1 1 1] Check if the user scrolled
    (if (not (== _returnvalue 0)) :!label _label
      (`/Game/InventorySystem/UMG/WBP_HotbarWidget.SetSelectedSlot` _hotbarwidget (+ (`/Game/InventorySystem/UMG/WBP_HotbarWidget.SelectedSlotID` _hotbarwidget) _returnvalue))))
  (:`Ongoing`
    (goto _label)))

(event `EnhancedInput|/Game/FP_Player/Input/DropItem`
  (params (ActionValue :type Boolean) (ElapsedSeconds :type "Float (double-precision)") (TriggeredSeconds :type "Float (double-precision)") (InputAction :type "InputAction Object Reference" :default "/Game/FP_Player/Input/DropItem.DropItem"))
  (bind _inventorymanager (`self.InventoryManager`))
  (bind _hotbarwidget (`/Game/InventorySystem/Blueprints/BP_InventoryManagerComponent.HotbarWidget` _inventorymanager))
  (bind _output (`|GetArrayItem` (`/Game/InventorySystem/UMG/WBP_HotbarWidget.HotbarSlots` _hotbarwidget) (`/Game/InventorySystem/UMG/WBP_HotbarWidget.SelectedSlotID` _hotbarwidget)))
  ;[1 1 1] The hotbar controls to operate everything to do with the hotbar!!!
  ;;[1 1 1] DoItemDropping
  ;;;[1 1 1] Drop a single item
  (:`Triggered`
    (`/Engine/EditorBlueprintResources/StandardMacros.IsValid` _output
      (:`Is Valid`
        (`/Game/InventorySystem/Blueprints/BP_InventoryManagerComponent.DropItemAtIndex` _inventorymanager (`/Game/InventorySystem/UMG/WBP_HotbarSlot.SlotID` _output) 1)))))

(event `EnhancedInput|/Game/FP_Player/Input/DropItems`
  (params (ActionValue :type Boolean) (ElapsedSeconds :type "Float (double-precision)") (TriggeredSeconds :type "Float (double-precision)") (InputAction :type "InputAction Object Reference" :default "/Game/FP_Player/Input/DropItems.DropItems"))
  (bind _inventorymanager (`self.InventoryManager`))
  (bind _hotbarwidget (`/Game/InventorySystem/Blueprints/BP_InventoryManagerComponent.HotbarWidget` _inventorymanager))
  (bind _output (`|GetArrayItem` (`/Game/InventorySystem/UMG/WBP_HotbarWidget.HotbarSlots` _hotbarwidget) (`/Game/InventorySystem/UMG/WBP_HotbarWidget.SelectedSlotID` _hotbarwidget)))
  ;[1 1 1] The hotbar controls to operate everything to do with the hotbar!!!
  ;;[1 1 1] DoItemDropping
  ;;;[1 1 1] Drop all remaining items
  (:`Triggered`
    (`/Engine/EditorBlueprintResources/StandardMacros.IsValid` _output
      (:`Is Valid`
        (`/Game/InventorySystem/Blueprints/BP_InventoryManagerComponent.DropItemAtIndex` _inventorymanager (`/Game/InventorySystem/UMG/WBP_HotbarSlot.SlotID` _output) -1)))))

(fn `customDelay`
  (params (time :type Integer))
  (for _index (range (stale _result) (+ time 1))
    (bind _result (`/Engine/EditorBlueprintResources/StandardMacros.IncrementInt` _index)
      (:`  `
        (return)))))

(fn `Destroy Pig`
  (params (Location :type "Transform Structure") (Actor :type "Actor Object Reference"))
  (set `self.temp transform` Location)
  (`|ExecutionSequence`
    (:`then_0`
      (`self.K2_DestroyActor` Actor))
    (:`then_1`
      (for _ (range (+ (`KismetMathLibrary.RandomIntegerInRange` 1 4) 1))
        (`|SpawnActorFromClass` "/Game/Blueprints/Items/Stone.Stone_C" (`self.temp transform`) "Undefined" "OverrideRootScale" null "NewEnumerator1" null)))))

(fn `Destroy Rock`
  (params (location :type "Transform Structure") (Actor :type "Actor Object Reference"))
  (set `self.temp transform` location)
  (`|ExecutionSequence`
    (:`then_0`
      (`self.K2_DestroyActor` Actor))
    (:`then_1`
      (for _index (range (+ (`KismetMathLibrary.RandomIntegerInRange` 1 4) 1))
        (`|SpawnActorFromClass` "/Game/Blueprints/Items/Stone.Stone_C" (`self.temp transform`) "Undefined" "OverrideRootScale" null "NewEnumerator1" null)))))

(fn `destroy tree`
  (params (Location :type "Transform Structure") (actor :type "Actor Object Reference"))
  (set `self.temp transform` Location)
  (`|ExecutionSequence`
    (:`then_0`
      (`self.K2_DestroyActor` actor))
    (:`then_1`
      (for _index (range (+ (`KismetMathLibrary.RandomIntegerInRange` 1 4) 1))
        (`|SpawnActorFromClass` "/Game/Blueprints/Items/Wood.Wood_C" (`self.temp transform`) "Undefined" "OverrideRootScale" null "NewEnumerator0" null)
        (`/Engine/EditorBlueprintResources/StandardMacros.IncrementInt` _index)))))

(fn `Start Crouching`
  (`self.Crouch`)
  (set `self.Is Crouching` true))

(fn `Start Sprinting`
  (set `CharacterMovementComponent.MaxWalkSpeed` 900.0 (`self.CharacterMovement`))
  (set `self.Is Sprinting` true))

(fn `Stop Crouching`
  (`self.UnCrouch`)
  (set `self.Is Crouching` false))

(fn `Stop Sprinting`
  (set `CharacterMovementComponent.MaxWalkSpeed` 600.0 (`self.CharacterMovement`))
  (set `self.Is Sprinting` false))

(fn `tag checker`
  (params (actor :type "Actor Object Reference"))
  (returns (Tag :type Name) (`actor out` :type "Actor Object Reference"))
  (`|ExecutionSequence`
    (:`then_0`
      (if (`self.ActorHasTag` actor "Tree")
        (return "tree" actor)))
    (:`then_1`
      (if (`self.ActorHasTag` actor "Rock")
        (return "Rock" actor)))
    (:`then_2`
      (if (`self.ActorHasTag` actor "Pig")
        (return "Pig" actor)))))

(fn `Useable_actor`
  (returns (UsableActor :type "/Game/Code/BP_UsableActor Object Reference"))
  (bind (_returnvalue_x _returnvalue_y _returnvalue_z) (`KismetMathLibrary.BreakVector` (`SceneComponent.K2_GetComponentLocation` (`self.Camera`))))
  (bind _returnvalue (+ (`self.K2_GetActorLocation`) (`KismetMathLibrary.MakeVector` 0.0 0.0 _returnvalue_z)))
  ;[1 1 1] Eye Location
  (bind _outhit (`KismetSystemLibrary.LineTraceSingleForObjects` _returnvalue (+ _returnvalue (* (`SceneComponent.GetForwardVector` (`self.Camera`)) 100.0)) (`|MakeArray` "ObjectTypeQuery1" "ObjectTypeQuery2" :!type "EObjectTypeQuery Enum")))
  (bind _asbp_usable_actor (cast `/Game/Code/BP_UsableActor` (`.HitActor` (`GameplayStatics.BreakHitResult` _outhit)))
    (:`then`
      _)
    (:`CastFailed`
      _))
  (return _asbp_usable_actor))

(fn `UserConstructionScript`)