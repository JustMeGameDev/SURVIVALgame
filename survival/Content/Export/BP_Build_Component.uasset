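; Build-mode component for BP_Character2 that previews and spawns buildable items loaded from DTBP_Items by type.
; While active, a 0.01-second delay loop line-traces from the camera on the item's channel to position a collisionless ghost mesh.
; The ghost snaps to hit build boxes; one trace channel also permits free placement.
; A bounds-sized box trace checks overlap, setting CanBuild and green/red materials; SpawnBuild spawns the actor at that transform.
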(event `self.ReceiveBeginPlay`
  (bind _asbp_character_2 (cast `/Game/FP_Player/BP_Character2` (`self.GetOwner`)))
  (set `self.playerRef` _asbp_character_2)
  (bind _outrownames (`DataTableFunctionLibrary.GetDataTableRowNames` "/Game/Export/NewFolder/DTBP_Items.DTBP_Items"))
  (for _array_element _outrownames
    (bind _returnvalue (`|GetDataTableRow` "/Game/Export/NewFolder/DTBP_Items.DTBP_Items" _array_element)
      (:`then`
        (if (`|EnumEquality` (`.Types_5_EB643334433BBBB6539C93A5D76984B3` (break `/Game/Export/STBP_Item` _returnvalue)) "NewEnumerator3")
          (`KismetArrayLibrary.Array_Add` (`self.buildables`) _returnvalue))))))

(event `BuildDelay`
  (bind _buildghost (`self.buildGhost`))
  (if (`self.isBuildModeOn`)
    (`KismetSystemLibrary.Delay` 0.01)
    (`self.BuildCycle`)
    (else
      (set `self.isBuildModeOn` false :!label _label)
      (set `self.canBuild` false)
      (`/Engine/EditorBlueprintResources/StandardMacros.IsValid` _buildghost
        (:`Is Valid`
          (`self.K2_DestroyComponent` _buildghost))))))

(event `StopBuildMode`
  (goto _label))

(event `LaunchBuildMode`
  (if (`self.isBuildModeOn`)
    (`self.StopBuildMode`)
    (else
      (set `self.isBuildModeOn` true)
      (`self.BuildCycle`))))

(fn `BuildCycle`
  (bind _camera (`self.camera`))
  (bind (_buildtransform_location _buildtransform_rotation _buildtransform_scale) (`KismetMathLibrary.BreakTransform` (`self.buildTransform`)))
  (bind _buildghost (`self.buildGhost`))
  (bind _returnvalue (`SceneComponent.K2_GetComponentLocation` _camera))
  (bind _returnvalue_2 (`SceneComponent.GetForwardVector` _camera))
  (bind (_output_name _output_types _output_description _output_icon _output_model _output_rarity _output_quantity _output_stackable _output_tracechannel) (break `/Game/Export/STBP_Item` (`|GetArrayItem` (`self.buildables`) (`self.buildID`))))
  (bind (_outhit _returnvalue_3) (`KismetSystemLibrary.LineTraceSingle` (+ _returnvalue (* _returnvalue_2 25)) (+ _returnvalue (* _returnvalue_2 1000)) _output_tracechannel))
  (if _returnvalue_3
    (bind (_bblockinghit _binitialoverlap _time _distance _location _impactpoint _normal _impactnormal _physmat _hitactor _hitcomponent _hitbonename _bonename _hititem _elementindex _faceindex _tracestart _traceend) (`GameplayStatics.BreakHitResult` _outhit))
    (set `self.buildTransform` (`KismetMathLibrary.MakeTransform` _impactpoint _buildtransform_rotation _buildtransform_scale))
    (set `self.Hit Actor` _hitactor)
    (set `self.Hit Component` _hitcomponent)
    (`/Engine/EditorBlueprintResources/StandardMacros.IsValid` _buildghost
      (:`Is Valid`
        (bind (_found _transform) (`self.DetectBuildBoxes`))
        (if _found
          (set `self.buildTransform` _transform)
          (bind _hit (`self.CheckForOverlap` :!label _label))
          (if _hit
            (`self.GiveBuildColour` false :!label _label_2)
            (else
              (`self.GiveBuildColour` true)))
          (elif (`|EnumEquality` "TraceTypeQuery4" _output_tracechannel)
            (goto _label)
            (else
              (goto _label_2))))
        (`self.BuildDelay`))
      (:`Is Not Valid`
        (`self.SpawnBuildGhost` :!label _label_3)
        (`self.BuildDelay` :!label _label_4)))
    (else
      (set `self.buildTransform` (`KismetMathLibrary.MakeTransform` _traceend _buildtransform_rotation _buildtransform_scale))
      (`/Engine/EditorBlueprintResources/StandardMacros.IsValid` _buildghost
        (:`Is Valid`
          (`self.GiveBuildColour` false)
          (goto _label_4))
        (:`Is Not Valid`
          (goto _label_3))))))

(fn `ChangeMesh`
  (bind (_output_name _output_types _output_description _output_icon _output_model) (break `/Game/Export/STBP_Item` (`|GetArrayItem` (`self.buildables`) (`self.buildID`))))
  (`StaticMeshComponent.SetStaticMesh` (`self.buildGhost`) _output_model))

(fn `CheckForOverlap`
  (returns (hit :type Boolean))
  (bind (_origin _boxextent) (`KismetSystemLibrary.GetComponentBounds` (`self.buildGhost`)))
  (bind (_outhit _returnvalue) (`KismetSystemLibrary.BoxTraceSingle` _origin _origin _boxextent (struct) "TraceTypeQuery1"))
  (return _returnvalue))

(fn `DetectBuildBoxes`
  (returns (found :type Boolean) (transform :type "Transform Structure"))
  (locals (localFound :type Boolean))
  (bind _boxes (message `/Game/Interfaces/I_BP_BuildInterface.ReturnBoxes` (`self.Hit Actor`)))
  (for _array_element _boxes
    (if (== _array_element (`self.Hit Component`))
      (set `local.localFound` true)
      (break)))
  (return (`local.localFound`) (`SceneComponent.K2_GetComponentToWorld` (`self.Hit Component`))))

(fn `GiveBuildColour`
  (params (isGreen :type Boolean))
  (set `self.canBuild` isGreen)
  (for _index (range (`PrimitiveComponent.GetNumMaterials` (`self.buildGhost`)))
    (if isGreen
      (`PrimitiveComponent.SetMaterial` (`self.buildGhost`) _index "/Game/Materials/GreenColour.GreenColour")
      (else
        (`PrimitiveComponent.SetMaterial` (`self.buildGhost`) _index "/Game/Materials/RedColour.RedColour"))))
  (`SceneComponent.K2_SetWorldTransform` (`self.buildGhost`) (`self.buildTransform`) false false))

(fn `Spawn Build`
  (bind (_output_name _output_types _output_description _output_icon _output_model _output_rarity _output_quantity _output_stackable _output_tracechannel _output_actor) (break `/Game/Export/STBP_Item` (`|GetArrayItem` (`self.buildables`) (`self.buildID`))))
  (bind _returnvalue (`|SpawnActorFromClass` _output_actor (`self.buildTransform`) "Undefined" "OverrideRootScale" null null))
  (message `/Game/Interfaces/I_BP_BuildInterface.SetMesh` _returnvalue _output_model))

(fn `SpawnBuildGhost`
  (bind (_output_name _output_types _output_description _output_icon _output_model) (break `/Game/Export/STBP_Item` (`|GetArrayItem` (`self.buildables`) (`self.buildID`))))
  (bind _returnvalue (`|AddComponentByClass` (`self.playerRef`) "/Script/Engine.StaticMeshComponent" false (`self.buildTransform`)))
  (bind _output_get (set `self.buildGhost` _returnvalue))
  (`StaticMeshComponent.SetStaticMesh` _output_get _output_model)
  (`PrimitiveComponent.SetCollisionEnabled` (`self.buildGhost`) "NoCollision"))