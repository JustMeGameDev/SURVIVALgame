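; BP_UseAppel is the use logic for an apple item that restores the player's food and water.
; On BeginPlay it caches the player's BP_Character2.
; Its used event runs a two-step sequence that adds a fixed amount to Fod and Water, each clamped to its maximum and skipped when full.
; Either successful step prints the new value after a short delay and destroys the actor, so nothing is consumed when both are full.
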(event `self.ReceiveBeginPlay`
  (bind _asbp_character_2 (cast `/Game/FP_Player/BP_Character2` (`GameplayStatics.GetPlayerCharacter` 0)))
  (set `self.NewVar` _asbp_character_2)
  (`KismetSystemLibrary.PrintString` "cast succes"))

(event `used`
  (bind _newvar (`self.NewVar`))
  (bind _newvar_2 (`self.NewVar`))
  (bind _newvar_3 (`self.NewVar`))
  (bind _maxfod (`/Game/FP_Player/BP_Character2.MaxFod` _newvar_2))
  (bind _maxwater (`/Game/FP_Player/BP_Character2.MaxWater` _newvar_3))
  (`|ExecutionSequence`
    (:`then_0`
      (bind _output_get (set `self.NewVar_0` (>= (`/Game/FP_Player/BP_Character2.Fod` _newvar_2) _maxfod)))
      (if (not _output_get)
        (bind _output_get_2 (set `/Game/FP_Player/BP_Character2.Fod` (`KismetMathLibrary.Clamp` (+ (`/Game/FP_Player/BP_Character2.Fod` _newvar_2) 5) 0 _maxfod) _newvar_3))
        (`KismetSystemLibrary.Delay` 0.5)
        (`KismetSystemLibrary.PrintString` (`KismetStringLibrary.Conv_IntToString` _output_get_2))
        (`self.K2_DestroyActor` self)))
    (:`then_1`
      (bind _output_get_3 (set `self.NewVar_1` (>= (`/Game/FP_Player/BP_Character2.water` _newvar_3) _maxwater)))
      (if (not _output_get_3)
        (bind _output_get_4 (set `/Game/FP_Player/BP_Character2.water` (`KismetMathLibrary.Clamp` (+ (`/Game/FP_Player/BP_Character2.water` _newvar) 5) 0 _maxwater) _newvar))
        (`KismetSystemLibrary.Delay` 0.5)
        (`KismetSystemLibrary.PrintString` (`KismetStringLibrary.Conv_IntToString` _output_get_4))
        (`self.K2_DestroyActor` self)))))

(fn `UserConstructionScript`)